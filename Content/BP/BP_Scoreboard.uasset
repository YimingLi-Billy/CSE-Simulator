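; BP_Scoreboard is an in-world scoreboard that shows the game state's Score through a widget component.
; On BeginPlay it casts the game state to CSEGameState and the component's user widget to CustomScoreboard, then writes a "Score" label and the value into its text fields.
; The score is read only once, with no Tick or event updates, and debug strings print on start and on a failed widget cast.
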(event `self.ReceiveBeginPlay`
  (`KismetSystemLibrary.PrintString` "Hello")
  (bind _ascsegame_state (cast `/Game/CSEGameState` (`GameplayStatics.GetGameState`)))
  (bind _ascustom_scoreboard (cast `/Game/BP/CustomScoreboard` (`WidgetComponent.GetUserWidgetObject` (`self.GetComponentByClass` "/Script/UMG.WidgetComponent")))
    (:`then`
      (`TextBlock.SetText` (`/Game/BP/CustomScoreboard.Info` _ascustom_scoreboard) "Score")
      (`TextBlock.SetText` (`/Game/BP/CustomScoreboard.Score` _ascustom_scoreboard) (`KismetTextLibrary.Conv_IntToText` (`/Game/CSEGameState.score` _ascsegame_state))))
    (:`CastFailed`
      (`KismetSystemLibrary.PrintString` "Failed"))))

(fn `UserConstructionScript`)